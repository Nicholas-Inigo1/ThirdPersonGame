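; Elevator platform actor that moves its mesh along a timeline once the third-person character steps into its collision volume.
; Collision overlaps toggle an on-button flag and print a debug message on entry, while Tick calls Play on the timeline whenever the flag is set.
; The timeline drives the mesh's relative location without sweep.
; Leaving only clears the flag, with no stop or reverse.
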(event `self.Collision.OnComponentBeginOverlap`
  (params (OverlappedComponent :type "PrimitiveComponent Object Reference") (OtherActor :type "Actor Object Reference") (OtherComp :type "PrimitiveComponent Object Reference") (OtherBodyIndex :type Integer) (bFromSweep :type Boolean) (SweepResult :type "HitResult Structure (by ref)"))
  (cast `/Game/ThirdPerson/Blueprints/BP_ThirdPersonCharacter` OtherActor)
  (`KismetSystemLibrary.PrintString` "On Button")
  (set `self.PlayerOnButton` true))

(event `self.Collision.OnComponentEndOverlap`
  (params (OverlappedComponent :type "PrimitiveComponent Object Reference") (OtherActor :type "Actor Object Reference") (OtherComp :type "PrimitiveComponent Object Reference") (OtherBodyIndex :type Integer))
  (cast `/Game/ThirdPerson/Blueprints/BP_ThirdPersonCharacter` OtherActor)
  (set `self.PlayerOnButton` false))

(event `self.ReceiveTick`
  (params (DeltaSeconds :type "Float (single-precision)"))
  (if (`self.PlayerOnButton`)
    (bind (_direction _newtrack_2) (`Timeline|Timeline`)
      (:`Update`
        (`SceneComponent.K2_SetRelativeLocation` (`self.SM_ElevatorPlatform`) _newtrack_2 false false)))))

(fn `UserConstructionScript`)