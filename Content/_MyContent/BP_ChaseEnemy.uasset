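; Enemy character that chases the player and loses health when the player overlaps it, intended as a head-stomp hit.
; PawnSensing sets a sighting flag that is never cleared, after which Tick moves it straight toward player 0 and turns it to face them, without pathfinding.
; Any actor overlap with BP_ThirdPersonCharacter launches that character along LaunchDirection and removes one health, destroying the enemy at zero.
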(event `self.ReceiveTick`
  (params (DeltaSeconds :type "Float (single-precision)"))
  (if (`self.SeesPawn`)
    (`self.FollowPlayer`)))

(event `self.PawnSensing.OnSeePawn`
  (params (Pawn :type "Pawn Object Reference"))
  (set `self.SeesPawn` true))

(event `FollowPlayer`
  (bind (_returnvalue_x _returnvalue_y) (`KismetMathLibrary.BreakVector` (`self.K2_GetActorLocation`)))
  (bind (_returnvalue_x_2 _returnvalue_y_2) (`KismetMathLibrary.BreakVector` (`self.K2_GetActorLocation` (`GameplayStatics.GetPlayerPawn` 0))))
  ;[1 1 1] Follow Player
  (`self.AddMovementInput` (`KismetMathLibrary.Normal` (- (`self.K2_GetActorLocation` (`GameplayStatics.GetPlayerPawn` 0)) (`self.K2_GetActorLocation`))))
  (`self.K2_SetActorRotation` (`KismetMathLibrary.FindLookAtRotation` (`KismetMathLibrary.MakeVector` _returnvalue_x _returnvalue_y) (`KismetMathLibrary.MakeVector` _returnvalue_x_2 _returnvalue_y_2))))

(event `self.ReceiveActorBeginOverlap`
  (params (OtherActor :type "Actor Object Reference"))
  ;[1 1 1] Head Collision
  (bind _asbp_third_person_character (cast `/Game/ThirdPerson/Blueprints/BP_ThirdPersonCharacter` OtherActor))
  (`self.LaunchCharacter` _asbp_third_person_character (`self.LaunchDirection`) false false)
  (set `self.Healh` (- (`self.Healh`) 1))
  (if (<= (`self.Healh`) 0)
    (`self.K2_DestroyActor`)))

(fn `UserConstructionScript`)