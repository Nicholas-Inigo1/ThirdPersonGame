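; BP_FakePlatform is a trap platform that vanishes shortly after the third-person character touches it, then returns.
; A box overlap by any actor brightens a dynamic material and flip-flops a timeline between playing and reversing to animate opacity.
; After a short delay, a character cast gates hiding the mesh and disabling its collision.
; A second delay restores visibility, collision and the unlit brightness value.
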(event `self.ReceiveBeginPlay`
  (bind _returnvalue (`PrimitiveComponent.CreateDynamicMaterialInstance` (`self.SM_FakePlatform`) 0 "/Game/_MyContent/M_Bright.M_Bright" "None"))
  (bind _output_get (set `self.DynamicMaterial` _returnvalue))
  (`MaterialInstanceDynamic.SetScalarParameterValue` _output_get "Bright" 0.0))

(event `self.Box.OnComponentBeginOverlap`
  (params (OverlappedComponent :type "PrimitiveComponent Object Reference") (OtherActor :type "Actor Object Reference") (OtherComp :type "PrimitiveComponent Object Reference") (OtherBodyIndex :type Integer) (bFromSweep :type Boolean) (SweepResult :type "HitResult Structure (by ref)"))
  (`MaterialInstanceDynamic.SetScalarParameterValue` (`self.DynamicMaterial`) "Bright" 10.0)
  (`|ExecutionSequence`
    (:`then_0`
      (`/Engine/EditorBlueprintResources/StandardMacros.FlipFlop`
        (:`A`
          (bind (_direction _newtrack_0) (`Timeline|Timeline` :!label _label)
            (:`Update`
              (`MaterialInstanceDynamic.SetScalarParameterValue` (`self.DynamicMaterial`) "Opacity" _newtrack_0))))
        (:`B`
          (goto _label :!via `Reverse`))))
    (:`then_2`
      (`KismetSystemLibrary.Delay` 1.0)
      (cast `/Game/ThirdPerson/Blueprints/BP_ThirdPersonCharacter` OtherActor)
      (`SceneComponent.SetVisibility` (`self.SM_FakePlatform`) false false)
      (`PrimitiveComponent.SetCollisionEnabled` (`self.SM_FakePlatform`) "NoCollision")
      (`KismetSystemLibrary.Delay` 3.0)
      (`SceneComponent.SetVisibility` (`self.SM_FakePlatform`) true false)
      (`PrimitiveComponent.SetCollisionEnabled` (`self.SM_FakePlatform`) "QueryAndPhysics")
      (`MaterialInstanceDynamic.SetScalarParameterValue` (`self.DynamicMaterial`) "Bright" 0.0))))

(fn `UserConstructionScript`)